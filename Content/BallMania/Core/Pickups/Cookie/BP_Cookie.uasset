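; BP_Cookie is a cookie pickup actor that picks a random cookie variant when it spawns.
; On BeginPlay it sets a random spin rate on its RotatingMovement component and makes a weighted roll over the ECookieStats array.
; SummonValues totals the weights, and DetermineIndex walks the running sum to find the rolled entry.
; The selected entry is stored in SelectedCookie and supplies the materials for the base and chip meshes.
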(event `self.ReceiveBeginPlay`
  (set `RotatingMovementComponent.RotationRate` (`KismetMathLibrary.MakeRotator` 0.0 0.0 (`KismetMathLibrary.RandomFloatInRange` 180.0 360.0)) (`self.RotatingMovement`))
  (bind _sum_of_values (`self.SummonValues`))
  (bind _index (`self.DetermineIndex` (`KismetMathLibrary.RandomFloatInRange` 0.0 _sum_of_values)))
  (bind _output_get (set `self.SelectedCookie` (`|GetArrayItem` (`self.E_CookieStats`) _index)))
  (`PrimitiveComponent.SetMaterial` (`self.CookieBase`) 0 (break `/Game/BallMania/Core/Pickups/Cookie/S_CookieStats` _output_get))
  (`PrimitiveComponent.SetMaterial` (`self.CookieChips`) 0 (`.ChipMaterial_15_2319D81D4EA2676C3174658F535C52F8` (break `/Game/BallMania/Core/Pickups/Cookie/S_CookieStats` _output_get))))

(fn `DetermineIndex`
  (params (`Random Value` :type "Float (double-precision)"))
  (returns (Index :type Integer))
  (locals (`Local Sum` :type "Float (double-precision)"))
  (for (_array_element _array_index) (`self.E_CookieStats`)
    (bind _output_get (set `local.Local Sum` (+ (`.Weight_16_47D71EB3418AD7D2E3AF77B724861771` (break `/Game/BallMania/Core/Pickups/Cookie/S_CookieStats` _array_element)) (`local.Local Sum`))))
    (if (>= _output_get `Random Value`)
      (break)))
  (return _array_index))

(fn `SpawnCookie`)

(fn `SummonValues`
  (returns (`Sum Of Values` :type "Float (double-precision)"))
  (locals (LocalSum :type "Float (double-precision)"))
  (for _array_element (`self.E_CookieStats`)
    (set `local.LocalSum` (+ (`.Weight_16_47D71EB3418AD7D2E3AF77B724861771` (break `/Game/BallMania/Core/Pickups/Cookie/S_CookieStats` _array_element)) (`local.LocalSum`))))
  (return (`local.LocalSum`)))

(fn `UserConstructionScript`)