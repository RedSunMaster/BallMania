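; Game State for the Cookie Run game mode that runs the match countdown and decides the winner.
; On BeginPlay it copies the game length from BP_CookieRun_GM and starts a looping one-second timer, printing the remaining time each tick.
; When time runs out, it prints each Player State's points, picks the highest scorer, passes it to the Game Mode's CallGameEnded and pauses the game.
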(event `self.ReceiveBeginPlay`
  (bind _asbp_cookie_run_gm (cast `/Game/BallMania/Core/Gamemodes/CookieRun/BP_CookieRun_GM` (`GameplayStatics.GetGameMode`)))
  (bind _output_get (set `self.As BP Cookie Run GM` _asbp_cookie_run_gm))
  (set `self.GS_GameLength` (`/Game/BallMania/Core/Gamemodes/CookieRun/BP_CookieRun_GM.gameLength` _output_get))
  (bind _returnvalue (`KismetSystemLibrary.K2_SetTimerDelegate` (delegate `CountDown`) 1.0 true))
  (set `self.GameInProgress` _returnvalue))

(event `CountDown`
  (`KismetSystemLibrary.PrintString` (`KismetStringLibrary.Conv_DoubleToString` (`self.GS_GameLength`)))
  (`/Engine/EditorBlueprintResources/StandardMacros.DecrementFloat` (`self.GS_GameLength`)
    (:`  `
      (if (< (`self.GS_GameLength`) 0.0)
        (`KismetSystemLibrary.K2_ClearAndInvalidateTimerHandle` (`self.GameInProgress`))
        (for _array_element (`self.PlayerArray`)
          (bind _asbp_cookie_run_ps (cast `/Game/BallMania/Core/Gamemodes/CookieRun/BP_CookieRun_PS` _array_element))
          (bind _playerpoints (`/Game/BallMania/Core/Gamemodes/CookieRun/BP_CookieRun_PS.PlayerPoints` _asbp_cookie_run_ps))
          (`KismetSystemLibrary.PrintString` (`KismetStringLibrary.Concat_StrStr` (`KismetSystemLibrary.GetDisplayName` _asbp_cookie_run_ps) "      " (`KismetStringLibrary.Conv_DoubleToString` _playerpoints)) true true (struct :`G` 0.66 :`B` 1.0 :`A` 1.0) 100.0)
          (if (> _playerpoints (`self.currentWinningPoints`))
            (set `self.WinningPlayer` _asbp_cookie_run_ps)
            (set `self.currentWinningPoints` _playerpoints)))
        (`/Game/BallMania/Core/Gamemodes/BP_Base_GM.gameEnded` (`self.As BP Cookie Run GM`) (`self.WinningPlayer`))
        (`GameplayStatics.SetGamePaused` true)))))

(fn `UserConstructionScript`)