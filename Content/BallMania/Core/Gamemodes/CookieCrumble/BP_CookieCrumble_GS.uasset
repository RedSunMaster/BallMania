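; Game State for the Cookie Crumble game mode that detects the last player standing and ends the match.
; BeginPlay caches the Cookie Crumble Game Mode.
; checkAlivePlayers loops over PlayerArray, adding living players to AlivePlayers without clearing it first, and removing by loop index for dead ones.
; When exactly one entry remains, it passes that player to the Game Mode's CallGameEnded and pauses the game.
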(event `self.ReceiveBeginPlay`
  (bind _asbp_cookie_crumble_gm (cast `/Game/BallMania/Core/Gamemodes/CookieCrumble/BP_CookieCrumble_GM` (`GameplayStatics.GetGameMode`)))
  (set `self.gameModeReference` _asbp_cookie_crumble_gm))

(event `checkAlivePlayers`
  (bind _aliveplayers (`self.alivePlayers`))
  (bind _aliveplayers_2 (`self.alivePlayers`))
  (for (_array_element _array_index) (`self.PlayerArray`)
    (bind _asbp_cookie_crumble_ps (cast `/Game/BallMania/Core/Gamemodes/CookieCrumble/BP_CookieCrumble_PS` _array_element))
    (if (`/Game/BallMania/Core/Gamemodes/CookieCrumble/BP_CookieCrumble_PS.isPlayerAlive` _asbp_cookie_crumble_ps)
      (`KismetArrayLibrary.Array_Add` _aliveplayers _asbp_cookie_crumble_ps)
      (else
        (`KismetArrayLibrary.Array_Remove` _aliveplayers _array_index))))
  (if (== (`KismetArrayLibrary.Array_Length` _aliveplayers_2) 1)
    (`/Game/BallMania/Core/Gamemodes/BP_Base_GM.gameEnded` (`self.gameModeReference`) (`|GetArrayItem` _aliveplayers_2))
    (`GameplayStatics.SetGamePaused` true)))

(fn `UserConstructionScript`)