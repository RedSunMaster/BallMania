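; BP_Base_GM is the BallMania base game mode that sets up local multiplayer and announces the winner.
; After a short delay on BeginPlay, it loops over every PlayerStart, creating local players and giving each the default Enhanced Input mapping context.
; It spawns and possesses a BP_Character at each start, using the existing first controller for index zero.
; A bound GameEnded event prints the winning player's name as debug text.
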(event `self.ReceiveBeginPlay`
  (add `self.gameEnded` (delegate `Game Ended`))
  (`KismetSystemLibrary.Delay` 1.0)
  (bind _outactors (`GameplayStatics.GetAllActorsOfClass` "/Script/Engine.PlayerStart"))
  (for (_array_element _array_index) _outactors
    (bind _output_get (set `self.Array Index` _array_index))
    (bind _returnvalue (`GameplayStatics.CreatePlayer` _output_get))
    (if (> _array_index 0)
      (`EnhancedInputSubsystemInterface.AddMappingContext` (pcsubsystem `EnhancedInputLocalPlayerSubsystem` _returnvalue) "/Game/BallMania/Core/Engine/Inputs/IMC_Default.IMC_Default" 0 (struct))
      (bind _returnvalue_2 (`self.GetTransform` _array_element))
      (bind _returnvalue_3 (`|SpawnActorFromClass` "/Game/BallMania/Core/Characters/BP_Character.BP_Character_C" _returnvalue_2 "Undefined" "MultiplyWithRoot" null null))
      (`Controller.Possess` (`GameplayStatics.GetPlayerController` (`self.Array Index`)) _returnvalue_3)
      (else
        (`EnhancedInputSubsystemInterface.AddMappingContext` (pcsubsystem `EnhancedInputLocalPlayerSubsystem` (`GameplayStatics.GetPlayerController` 0)) "/Game/BallMania/Core/Engine/Inputs/IMC_Default.IMC_Default" 0 (struct))
        (bind _returnvalue_4 (`|SpawnActorFromClass` "/Game/BallMania/Core/Characters/BP_Character.BP_Character_C" _returnvalue_2 "Undefined" "MultiplyWithRoot" null null))
        (`Controller.Possess` (`GameplayStatics.GetPlayerController` 0) _returnvalue_4)))))

(event `Game Ended` :!signature `self.gameEnded`
  (params (`Winning Player` :type "PlayerState Object Reference"))
  (`KismetSystemLibrary.PrintString` "Game Has Ended")
  (`KismetSystemLibrary.PrintString` (`KismetStringLibrary.Concat_StrStr` (`KismetSystemLibrary.GetDisplayName` `Winning Player`) " Has Won!") true true (struct :`G` 0.66 :`B` 1.0 :`A` 1.0) 100.0))

(fn `UserConstructionScript`)