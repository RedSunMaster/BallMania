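; Placeable spawner that builds a square grid of BP_BreakawayFloor tiles for Ball Mania when play begins.
; Nested loops over FloorSize place tiles at a fixed spacing, centered on the root component's location at its height.
; Each column's first tile spawns separately, and its Y omits the root's world Y, so that edge only lines up when the spawner sits at Y zero.
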(event `self.ReceiveBeginPlay`
  (bind (_returnvalue_x _returnvalue_y _returnvalue_z) (`KismetMathLibrary.BreakVector` (`SceneComponent.K2_GetComponentLocation` (`self.DefaultSceneRoot`))))
  (set `self.leftPoint` (* (/ (* (- (`self.floorSize`) 1) 110) 2.0) -1.0))
  (for _index (range (`self.floorSize`))
    (bind _returnvalue (+ (+ (* _index 110) (`self.leftPoint`)) _returnvalue_x))
    (`|SpawnActorFromClass` "/Game/BallMania/Placeables/BreakawayFloor/BP_BreakawayFloor.BP_BreakawayFloor_C" (`KismetMathLibrary.MakeTransform` (`KismetMathLibrary.MakeVector` _returnvalue (`self.leftPoint`) _returnvalue_z)) "Undefined" "MultiplyWithRoot" null null)
    (for _index_2 (range 1 (`self.floorSize`))
      (`|SpawnActorFromClass` "/Game/BallMania/Placeables/BreakawayFloor/BP_BreakawayFloor.BP_BreakawayFloor_C" (`KismetMathLibrary.MakeTransform` (`KismetMathLibrary.MakeVector` _returnvalue (+ (+ (* _index_2 110) _returnvalue_y) (`self.leftPoint`)) _returnvalue_z)) "Undefined" "MultiplyWithRoot" null null))))

(fn `UserConstructionScript`)