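; BP_BreakawayEliminationZone is a trigger volume that eliminates players who enter it in the Cookie Crumble mode.
; On box overlap by a BP_Character, it marks the player state as not alive, notifies BP_CookieCrumble_GM of the elimination, then destroys the character.
; The construction script sizes the box collision from the Area variable, so each placed zone can be scaled.
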(event `self.BoxCollision.OnComponentBeginOverlap`
  (params (OverlappedComponent :type "PrimitiveComponent Object Reference") (OtherActor :type "Actor Object Reference") (OtherComp :type "PrimitiveComponent Object Reference") (OtherBodyIndex :type Integer) (bFromSweep :type Boolean) (SweepResult :type "HitResult Structure (by ref)"))
  (bind _asbp_character (cast `/Game/BallMania/Core/Characters/BP_Character` OtherActor))
  (bind _asbp_cookie_crumble_ps (cast `/Game/BallMania/Core/Gamemodes/CookieCrumble/BP_CookieCrumble_PS` (`Pawn.PlayerState` _asbp_character)))
  (set `/Game/BallMania/Core/Gamemodes/CookieCrumble/BP_CookieCrumble_PS.isPlayerAlive` false _asbp_cookie_crumble_ps)
  (bind _asbp_cookie_crumble_gm (cast `/Game/BallMania/Core/Gamemodes/CookieCrumble/BP_CookieCrumble_GM` (`GameplayStatics.GetGameMode`)))
  (`/Game/BallMania/Core/Gamemodes/CookieCrumble/BP_CookieCrumble_GM.playerEliminated` _asbp_cookie_crumble_gm)
  (`self.K2_DestroyActor` _asbp_character))

(fn `UserConstructionScript`
  (`BoxComponent.SetBoxExtent` (`self.BoxCollision`) (`self.Area`) true))