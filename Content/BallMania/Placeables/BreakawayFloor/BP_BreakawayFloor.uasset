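; BP_BreakawayFloor is a placeable floor for BallMania that loses health while something overlaps it and eventually destroys itself.
; Overlapping the Collision component deals damage immediately and starts a looping timer for repeat hits, which is cleared when the overlap ends.
; Each hit recolours the floor through a dynamic material instance, indexing a colour array by remaining health, until health drops below zero.
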(event `self.ReceiveBeginPlay`
  (set `self.currentFloorHealth` (`self.maxFloorHealth`)))

(event `self.Collision.OnComponentBeginOverlap`
  (params (OverlappedComponent :type "PrimitiveComponent Object Reference") (OtherActor :type "Actor Object Reference") (OtherComp :type "PrimitiveComponent Object Reference") (OtherBodyIndex :type Integer) (bFromSweep :type Boolean) (SweepResult :type "HitResult Structure (by ref)"))
  (`KismetSystemLibrary.PrintString` "Overlapped")
  (`self.dealDamage`)
  (bind _returnvalue (`KismetSystemLibrary.K2_SetTimerDelegate` (delegate `dealDamage`) 1.0 true))
  (set `self.damageTimer` _returnvalue))

(event `dealDamage`
  (bind _output_get (set `self.currentFloorHealth` (- (`self.currentFloorHealth`) 1.0)))
  (if (< _output_get 0.0)
    (`self.K2_DestroyActor`)
    (else
      (bind _returnvalue (`PrimitiveComponent.CreateDynamicMaterialInstance` (`self.Floor`) 0 "/Game/BallMania/Placeables/BreakawayFloor/Materials/MI_BreakawayFloor.MI_BreakawayFloor" "None"))
      (`MaterialInstanceDynamic.SetVectorParameterValue` _returnvalue "FloorColour" (`|GetArrayItem` (`self.floorColours`) (`KismetMathLibrary.FTrunc` (`self.currentFloorHealth`)))))))

(event `self.Collision.OnComponentEndOverlap`
  (params (OverlappedComponent :type "PrimitiveComponent Object Reference") (OtherActor :type "Actor Object Reference") (OtherComp :type "PrimitiveComponent Object Reference") (OtherBodyIndex :type Integer))
  (`KismetSystemLibrary.PrintString` "Stopped Overlapping")
  (`KismetSystemLibrary.K2_ClearAndInvalidateTimerHandle` (`self.damageTimer`)))

(fn `UserConstructionScript`)